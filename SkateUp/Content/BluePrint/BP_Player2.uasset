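; BP_Player2 is a physics-driven player Blueprint moved by forces and velocity changes on its capsule.
; Enhanced Input drives controller yaw and pitch for looking, a Speed-scaled forward force for acceleration, and world-axis directional forces with X and Y swapped.
; Grab stops the capsule abruptly by zeroing linear velocity, and Tick prints velocity for debugging.
; An unconnected ragdoll setup for the skeletal mesh never runs.
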(event Input|EnhancedActionEvents|EnhancedInputActionIA_Accel
  (params (ActionValue :type Boolean) (ElapsedSeconds :type Float%20%28double-precision%29) (TriggeredSeconds :type Float%20%28double-precision%29) (InputAction :type Input%20Action%20Object%20Reference :default "/Game/Input/IA_Accel.IA_Accel"))
  ;[0.15 0.15 0.15 0.5] Speed 만큼의 힘을 전방 벡터 방향으로 Add
  (Physics|AddForce (Variables|Default|GetCapsule) (* (Transformation|GetActorForwardVector) (Variables|Default|GetSpeed)) "None" false))

(event Input|EnhancedActionEvents|EnhancedInputActionIA_Grab
  (params (ActionValue :type Boolean) (ElapsedSeconds :type Float%20%28double-precision%29) (TriggeredSeconds :type Float%20%28double-precision%29) (InputAction :type Input%20Action%20Object%20Reference :default "/Game/Input/IA_Grab.IA_Grab"))
  ;[0.15 0.15 0.15 0.5] Grab 트리거시 힘을 0으로 설정 (현재는 급정거)
  (Physics|SetPhysicsLinearVelocity (Variables|Default|GetCapsule) "0, 0, 0" false "None"))

(event Input|EnhancedActionEvents|EnhancedInputActionIA_DirectionMove
  (params (ActionValue :type Vector%202D%20Structure) (ElapsedSeconds :type Float%20%28double-precision%29) (TriggeredSeconds :type Float%20%28double-precision%29) (InputAction :type Input%20Action%20Object%20Reference :default "/Game/Input/IA_DirectionMove.IA_DirectionMove"))
  (bind _speed (Variables|Default|GetSpeed))
  (bind _returnvalue (* ActionValue _speed))
  ;[0.15 0.15 0.15 0.5] 코멘트
  (Physics|AddForce (Variables|Default|GetCapsule) (Math|Vector|MakeVector (.y _returnvalue) (.x _returnvalue) 0.0) "None" false))

(event Input|EnhancedActionEvents|EnhancedInputActionIA_Look
  (params (ActionValue :type Vector%202D%20Structure) (ElapsedSeconds :type Float%20%28double-precision%29) (TriggeredSeconds :type Float%20%28double-precision%29) (InputAction :type Input%20Action%20Object%20Reference :default "/Game/Input/IA_Look.IA_Look"))
  ;[0.15 0.15 0.15 0.5] 카메라 무빙 (폰 제어 회전 사용)
  (Pawn|Input|AddControllerYawInput (.x ActionValue))
  (Pawn|Input|AddControllerPitchInput (.y ActionValue)))

(event EventTick
  (params (DeltaSeconds :type Float%20%28single-precision%29))
  (Development|PrintString (Utilities|String|ToString(Vector) (Transformation|GetVelocity))))

(fn ConstructionScript)